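; BP_enemyShooting is a jumping enemy that fires BP_EnemyrProjectile and can be destroyed by damage.
; Tick drives two random Delays that act as repeating timers, one spawning projectiles at a fixed world-space offset with the actor's rotation, the other jumping.
; AnyDamage subtracts health, prints it and spawns an explosion, then destroys the actor at zero or below, with a DoOnce and Delay briefly ignoring further hits.
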(event EventBeginPlay
  (Variables|Default|SetCurrentHP (Variables|Default|GetMaxHP)))

(event Collision|EventActorBeginOverlap
  (params (OtherActor :type Actor%20Object%20Reference)))

(event EventTick
  (params (DeltaSeconds :type Float%20%28single-precision%29))
  (bind _returnvalue (Transformation|GetActorLocation))
  (Utilities|FlowControl|Sequence
    (:then_0
      (Utilities|FlowControl|Delay (Math|Random|RandomFloatinRange 1.0 5.0))
      (Game|SpawnActorfromClass "/Game/Enimies/BP_EnemyrProjectile.BP_EnemyrProjectile_C" (Math|Transform|MakeTransform (Math|Vector|MakeVector (.x _returnvalue) (+ (.y _returnvalue) 6e+01) (+ (.z _returnvalue) 2e+01)) (Transformation|GetActorRotation) "1,1,1") "AlwaysSpawn" 0 0))
    (:then_1
      (Utilities|FlowControl|Delay (Math|Random|RandomFloatinRange 3.0 8.0))
      (Character|Jump))))

(event Game|Damage|EventAnyDamage
  (params (Damage :type Float%20%28single-precision%29) (DamageType :type Damage%20Type%20Object%20Reference) (InstigatedBy :type Controller%20Object%20Reference) (DamageCauser :type Actor%20Object%20Reference))
  (Utilities|FlowControl|DoOnce false :!label _label
    (:Completed
      (bind _output_get (Variables|Default|SetCurrentHP (- (Variables|Default|GetCurrentHP) Damage)))
      (Development|PrintString (Utilities|String|ToString(Float) _output_get))
      (Effects|SpawnEmitteratLocation "/Game/StarterContent/Particles/P_Explosion.P_Explosion" (Transformation|GetActorLocation))
      (if (<= _output_get 0.0)
        (Actor|DestroyActor)
        (else
          (Utilities|FlowControl|Delay 0.5)
          (goto _label Reset))))))

(fn ConstructionScript
  (|CallParentFunction))