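; Falling carrot trap for the side-scroller that drops when the player crosses its trigger line and deals damage on contact.
; Each Tick it line-traces on the Camera channel to a Scene component placed at TraceEndPoint on BeginPlay.
; Hitting a SideScrollerCharacter starts physics on the Cone, enables the Sphere's overlap and destroys the actor after a delay.
; The Sphere applies damage to the character only once.
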(event OnComponentBeginOverlap(Sphere)
  (params (OverlappedComponent :type Primitive%20Component%20Object%20Reference) (OtherActor :type Actor%20Object%20Reference) (OtherComp :type Primitive%20Component%20Object%20Reference) (OtherBodyIndex :type Integer) (bFromSweep :type Boolean) (SweepResult :type Hit%20Result%20Structure%20%28by%20ref%29))
  (if (Variables|Default|GetIsFall)
    (bind _asside_scroller_character (Utilities|Casting|CastToSideScrollerCharacter OtherActor))
    (Utilities|FlowControl|DoOnce false
      (:Completed
        (Game|Damage|ApplyDamage _asside_scroller_character 1.0 0 0)))))

(event EventBeginPlay
  (Transformation|SetRelativeLocation (Variables|Default|GetScene) (Variables|Default|GetTraceEndPoint) false true)
  (Collision|SetCollisionEnabled (Variables|Default|GetSphere) "NoCollision"))

(event EventTick
  (params (DeltaSeconds :type Float%20%28single-precision%29))
  (if (not (Variables|Default|GetIsFall))
    (bind _outhit (Collision|LineTraceByChannel (Transformation|GetActorLocation) (Transformation|GetWorldLocation (Variables|Default|GetScene)) "TraceTypeQuery2" false 0 "None"))
    (if (.bBlockingHit (Collision|BreakHitResult _outhit))
      (Utilities|Casting|CastToSideScrollerCharacter (.HitActor (Collision|BreakHitResult _outhit)))
      (Variables|Default|SetIsFall true)
      (Physics|SetSimulatePhysics (Variables|Default|GetCone) true)
      (Collision|SetCollisionEnabled (Variables|Default|GetSphere) "QueryOnly")
      (Utilities|FlowControl|Delay 1e+01)
      (Actor|DestroyActor))))

(fn ConstructionScript)