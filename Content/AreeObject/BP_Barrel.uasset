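; BP_Barrel is a barrel hazard that damages the side-scroller character once it is activated.
; The overlap box starts without collision, so the barrel is harmless until BarrelActive runs.
; BarrelActive enables physics on the Cone component and query collision on the box, then destroys the actor after a delay.
; A DoOnce on the box overlap limits the damage to a single hit.
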(event OnComponentBeginOverlap(Box)
  (params (OverlappedComponent :type Primitive%20Component%20Object%20Reference) (OtherActor :type Actor%20Object%20Reference) (OtherComp :type Primitive%20Component%20Object%20Reference) (OtherBodyIndex :type Integer) (bFromSweep :type Boolean) (SweepResult :type Hit%20Result%20Structure%20%28by%20ref%29))
  (bind _asside_scroller_character (Utilities|Casting|CastToSideScrollerCharacter OtherActor))
  (Utilities|FlowControl|DoOnce false
    (:Completed
      (Game|Damage|ApplyDamage _asside_scroller_character 2.0 0 0))))

(event Custom|BarrelActive
  (Physics|SetSimulatePhysics (Variables|Default|GetCone) true)
  (Collision|SetCollisionEnabled (Variables|Default|GetBox) "QueryOnly")
  (Utilities|FlowControl|Delay 1e+01)
  (Actor|DestroyActor))

(event EventBeginPlay
  (Collision|SetCollisionEnabled (Variables|Default|GetBox) "NoCollision"))

(event EventTick
  (params (DeltaSeconds :type Float%20%28single-precision%29)))

(fn ConstructionScript)